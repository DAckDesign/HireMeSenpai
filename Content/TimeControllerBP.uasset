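; Time controller Blueprint that runs the interview and frenzy timers, plays soundtrack and reaction audio, and opens the pause menu.
; GameTimer starts alongside the music, while FrenzyTimer seeks to an offset derived from QuestionStartingTime and updates TimeLeft.
; Each timer notifies DialogueUI when it finishes.
; Escape or Shift+Escape pauses the game and creates GamePauseMenu, passing it whether the soundtrack is playing.
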(event `React`
  (params (ReactionSound :type "SoundWave Object Reference"))
  (bind _reactions (`self.Reactions`))
  (`AudioComponent.SetSound` _reactions ReactionSound)
  (`AudioComponent.Play` _reactions 0.0))

(event `StartGameTimer`
  (`|ExecutionSequence`
    (:`then_0`
      (`Timeline|GameTimer` :!via `PlayFromStart`
        (:`Finished`
          (`/Game/UI/Dialogue_UI.InterviewTimeOver` (`self.Dialogue_UI`)))))
    (:`then_1`
      (`AudioComponent.SetSound` (`self.Soundtrack`) "/Game/Audio/Soundtrack/Game_Audio_by_StereoSurgeon.Game_Audio_by_StereoSurgeon"))))

(event `StartFrenzyTimer`
  (`|ExecutionSequence`
    (:`then_0`
      (bind (_direction _timeleft) (`Timeline|FrenzyTimer` :`NewTime` (- 60.0 (`self.QuestionStartingTime`)) :!via `SetNewTime` :!label _label)
        (:`Update`
          (set `self.TimeLeft` _timeleft))
        (:`Finished`
          (`/Game/UI/Dialogue_UI.FrenzyTimeOver` (`self.Dialogue_UI`)))))
    (:`then_1`
      (goto _label))))

(event `StopTimer`
  (goto _label :!via `Stop`))

(event `Key|Escape`
  (params (Key :type "Key Structure"))
  (:`Pressed`
    (`GameplayStatics.SetGamePaused` true :!label _label_2)
    (bind _returnvalue (`|CreateWidget` "/Game/UI/GamePauseMenu.GamePauseMenu_C"))
    (bind _output_get (set `self.GamePauseMenu` _returnvalue))
    (set `/Game/UI/GamePauseMenu.MusicActive` (`AudioComponent.IsPlaying` (`self.Soundtrack`)) _output_get)
    (`UserWidget.AddToViewport` _output_get 0)))

(event `Key|Shift+Escape`
  (params (Key :type "Key Structure"))
  (:`Pressed`
    (goto _label_2)))

(fn `UserConstructionScript`)